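; BP_Enemy is a horror enemy whose looping audio follows gamma brainwave data from BP_MuseDataTransformer.
; Tick feeds the current gamma average through GammaLerper into the loop's GammaWaves parameter while lerping.
; Player overlap spawns a random jumpscare sound scaled by ScareIndicator, increments the game mode's loss count and destroys the enemy.
; SetGammaMinAndMax is bound to baseline calculation but empty; the gamma range setters are disconnected.
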(event OnComponentBeginOverlap(Trigger)
  (params (OverlappedComponent :type Primitive%20Component%20Object%20Reference) (OtherActor :type Actor%20Object%20Reference) (OtherComp :type Primitive%20Component%20Object%20Reference) (OtherBodyIndex :type Integer) (bFromSweep :type Boolean) (SweepResult :type Hit%20Result%20Structure%20%28by%20ref%29))
  ;[1 1 1] On Overlap
  (Utilities|Casting|CastToBP_Player OtherActor)
  (bind _returnvalue (Audio|SpawnSoundatLocation "/Game/Audio/MetaSounds/MS_Jumpscare.MS_Jumpscare" (Transformation|GetActorLocation) "0, 0, 0" 1.0 1.0 0.0 0 0))
  (Audio|Parameter|SetFloatParameter _returnvalue "ScareIndicator" (Variables|/Game/Blueprints/Muse/BP_MuseDataTransformer.BP_MuseDataTransformer_C|GetScareIndicator (Variables|Internal|GetREF_MuseDataTransformer)) :!class /Script/AudioExtensions.AudioParameterControllerInterface)
  (Audio|Parameter|SetObjectParameter _returnvalue "Wave Asset" (.OutItem (Utilities|Array|Random (Variables|Settings|GetJumpscareSounds))))
  (bind _asbp_game_mode (Utilities|Casting|CastToBP_GameMode (Game|GetGameMode)))
  (Default|IncrementLoss _asbp_game_mode)
  (Actor|DestroyActor))

(event Custom|SetGammaMinAndMax
  ;[1 1 1] Begin Play
)

(event EventBeginPlay
  ;[1 1 1] Begin Play
  (Audio|Components|Audio|FadeIn (Variables|Default|GetLoop) (Variables|Settings|GetFade%20in%20Duration) 1.0 0.0 "Linear" :!class /Script/Engine.AudioComponent)
  (bind _returnvalue (Actor|GetActorOfClass "/Game/Blueprints/Muse/BP_MuseDataTransformer.BP_MuseDataTransformer_C"))
  (bind _output_get (Variables|Internal|SetREF_MuseDataTransformer _returnvalue))
  (if (Variables|/Game/Blueprints/Muse/BP_MuseDataTransformer.BP_MuseDataTransformer_C|GetbIsBaselineCalculated _output_get)
    (CallFunction|SetGammaMinandMax))
  (EventDispatchers|BindEventtoOnBaselineCalculated _output_get (delegate Custom|SetGammaMinAndMax)))

(event EventTick
  (params (DeltaSeconds :type Float%20%28single-precision%29))
  (bind _gammalerper (Variables|Default|GetGammaLerper))
  ;[1 1 1] Tick
  (Default|SetTarget (Variables|Default|GetGammaLerper) (Variables|/Game/Blueprints/Muse/BP_MuseDataTransformer.BP_MuseDataTransformer_C|GetCurrentGammaAVG (Variables|Internal|GetREF_MuseDataTransformer)))
  (if (Variables|/Game/Blueprints/Components/BPC_FloatLerper.BPC_FloatLerper_C|GetbIsLerping _gammalerper)
    (Audio|Parameter|SetFloatParameter (Variables|Default|GetLoop) "GammaWaves" (Variables|/Game/Blueprints/Components/BPC_FloatLerper.BPC_FloatLerper_C|GetValue _gammalerper) :!class /Script/AudioExtensions.AudioParameterControllerInterface)))

(fn ConstructionScript)