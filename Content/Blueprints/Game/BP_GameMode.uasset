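; Game mode that tracks wins and losses and respawns the target and enemy near the player.
; Each respawn clears existing ones, picks random positive X/Y offsets from the player pawn, and re-rolls the enemy position until it is far enough from the target.
; When either counter reaches the shared threshold, it records the outcome in BP_GameInstance and opens the End level.
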(event EventBeginPlay)

(event EventTick
  (params (DeltaSeconds :type Float%20%28single-precision%29)))

(fn ConstructionScript)

(fn IncrementWin
  (bind _result (Math|Integer|IncrementInt (Variables|Game|GetWins))
    (:%20%20
      (if (>= _result (Variables|Settings|GetWinLoseThreshold))
        (Development|PrintString "You won!")
        (bind _asbp_game_instance (Utilities|Casting|CastToBP_GameInstance (Game|GetGameInstance)))
        (Variables|/Game/Blueprints/Game/BP_GameInstance.BP_GameInstance_C|SetWonGame _asbp_game_instance true)
        (Game|OpenLevel(byObjectReference) "/Game/Maps/Game/End.End")))))

(fn SpawnNewTargetandEnemyAroundPlayer
  (CallFunction|DestroyAllTargetsandEnemies)
  (bind _location (CallFunction|CalculateRandomLocationAroundPlayer))
  (LocalVariables|SetTargetLocation _location)
  (bind _location_2 (CallFunction|CalculateRandomLocationAroundPlayer))
  (LocalVariables|SetEnemyLocation _location_2)
  (while (< (Math|Vector|Distance(Vector) (LocalVariables|GetTargetLocation) (LocalVariables|GetEnemyLocation)) (Variables|Settings|GetMinDistanceBetweenObjects))
    (bind _location_3 (CallFunction|CalculateRandomLocationAroundPlayer))
    (LocalVariables|SetEnemyLocation _location_3))
  (Game|SpawnActorfromClass "/Game/Blueprints/Game/BP_Enemy.BP_Enemy_C" (Math|Transform|MakeTransform (LocalVariables|GetEnemyLocation) "0, 0, 0" "1.000000,1.000000,1.000000") "Undefined" 0 0)
  (Game|SpawnActorfromClass "/Game/Blueprints/Game/BP_Target.BP_Target_C" (Math|Transform|MakeTransform (LocalVariables|GetTargetLocation) "0, 0, 0" "1.000000,1.000000,1.000000") "Undefined" 0 0))

(fn CalculateRandomLocationAroundPlayer
  (return (+ (Transformation|GetActorLocation (Game|Player|GetPlayerPawn 0)) (Math|Vector|MakeVector (Math|Random|RandomFloatinRange 0.0 (Variables|Settings|GetMaxSpawnDistance)) (Math|Random|RandomFloatinRange 0.0 (Variables|Settings|GetMaxSpawnDistance)) 0.0))))

(fn IncrementLoss
  (bind _result (Math|Integer|IncrementInt (Variables|Game|GetLosses))
    (:%20%20
      (if (>= _result (Variables|Settings|GetWinLoseThreshold))
        (Development|PrintString "You Lost!")
        (bind _asbp_game_instance (Utilities|Casting|CastToBP_GameInstance (Game|GetGameInstance)))
        (Variables|/Game/Blueprints/Game/BP_GameInstance.BP_GameInstance_C|SetWonGame _asbp_game_instance false)
        (Game|OpenLevel(byObjectReference) "/Game/Maps/Game/End.End")))))

(fn DestroyAllTargetsandEnemies
  (bind _outactors (Actor|GetAllActorsOfClass "/Game/Blueprints/Game/BP_Target.BP_Target_C"))
  (for _array_element _outactors
    (Actor|DestroyActor _array_element))
  (bind _outactors_2 (Actor|GetAllActorsOfClass "/Game/Blueprints/Game/BP_Enemy.BP_Enemy_C"))
  (for _array_element_2 _outactors_2
    (Actor|DestroyActor _array_element_2)))