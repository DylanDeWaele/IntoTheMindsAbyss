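; BP_Target is a goal pickup whose audio responds to alpha brainwave data from BP_MuseDataTransformer.
; It fades in on spawn, then feeds the average alpha through a lerper into the sound's AlphaWaves parameter.
; Player overlap increments the game mode's win count, spawns a new target and enemy around the player, and destroys this one.
; The baseline-driven SetAlphaMinAndMax event is empty, leaving the AlphaMin/AlphaMax setters unconnected.
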(event OnComponentBeginOverlap(Trigger)
  (params (OverlappedComponent :type Primitive%20Component%20Object%20Reference) (OtherActor :type Actor%20Object%20Reference) (OtherComp :type Primitive%20Component%20Object%20Reference) (OtherBodyIndex :type Integer) (bFromSweep :type Boolean) (SweepResult :type Hit%20Result%20Structure%20%28by%20ref%29))
  ;[1 1 1] On Overlap
  (Utilities|Casting|CastToBP_Player OtherActor)
  (bind _asbp_game_mode (Utilities|Casting|CastToBP_GameMode (Game|GetGameMode)))
  (Default|IncrementWin _asbp_game_mode)
  (Default|SpawnNewTargetandEnemyAroundPlayer _asbp_game_mode)
  (Actor|DestroyActor))

(event Custom|SetAlphaMinAndMax
  ;[1 1 1] Begin Play
)

(event EventBeginPlay
  ;[1 1 1] Begin Play
  (Audio|Components|Audio|FadeIn (Variables|Default|GetAudio) (Variables|Settings|GetFade%20in%20Duration) 1.0 0.0 "Linear" :!class /Script/Engine.AudioComponent)
  (bind _returnvalue (Actor|GetActorOfClass "/Game/Blueprints/Muse/BP_MuseDataTransformer.BP_MuseDataTransformer_C"))
  (bind _output_get (Variables|Internal|SetREF_MuseDataTransformer _returnvalue))
  (if (Variables|/Game/Blueprints/Muse/BP_MuseDataTransformer.BP_MuseDataTransformer_C|GetbIsBaselineCalculated _output_get)
    (CallFunction|SetAlphaMinandMax))
  (EventDispatchers|BindEventtoOnBaselineCalculated _output_get (delegate Custom|SetAlphaMinAndMax)))

(event EventTick
  (params (DeltaSeconds :type Float%20%28single-precision%29))
  (bind _alphalerper (Variables|Default|GetAlphaLerper))
  (Default|SetTarget (Variables|Default|GetAlphaLerper) (Variables|/Game/Blueprints/Muse/BP_MuseDataTransformer.BP_MuseDataTransformer_C|GetCurrentAlphaAVG (Variables|Internal|GetREF_MuseDataTransformer)))
  (if (Variables|/Game/Blueprints/Components/BPC_FloatLerper.BPC_FloatLerper_C|GetbIsLerping _alphalerper)
    (Audio|Parameter|SetFloatParameter (Variables|Default|GetAudio) "AlphaWaves" (Variables|/Game/Blueprints/Components/BPC_FloatLerper.BPC_FloatLerper_C|GetValue _alphalerper) :!class /Script/AudioExtensions.AudioParameterControllerInterface)))

(fn ConstructionScript)