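; BP_Player is the player, moved by axis inputs and turned by input plus Muse gyroscope data.
; Each Tick it consumes movement input and sets its location directly, without sweep, scaled by MoveSpeed but not delta time.
; It also adds yaw from the Z gyroscope deviation of a BP_MuseDataTransformer found at BeginPlay.
; LookUp drives yaw, LookRight is empty, and both pitch paths are disconnected.
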(event EventBeginPlay
  ;[1 1 1] Begin Play
  (bind _returnvalue (Actor|GetActorOfClass "/Game/Blueprints/Muse/BP_MuseDataTransformer.BP_MuseDataTransformer_C"))
  (Variables|Default|SetREF_MuseDataTransformer _returnvalue))

(event EventTick
  (params (DeltaSeconds :type Float%20%28single-precision%29))
  (bind _ref_musedatatransformer (Variables|Default|GetREF_MuseDataTransformer))
  ;[1 1 1] CONSUMING INPUT
  (bind _returnvalue (Class|Pawn|ConsumeMovementInputVector))
  (Transformation|SetActorLocation (+ (Transformation|GetActorLocation) (* _returnvalue (Variables|Settings|GetMoveSpeed))) false false)
  (Utilities|IsValid _ref_musedatatransformer
    (:Is%20Valid
      (Pawn|Input|AddControllerYawInput (* (/ (.Z (Class|KismetMathLibrary|BreakVector3f (Variables|/Game/Blueprints/Muse/BP_MuseDataTransformer.BP_MuseDataTransformer_C|GetGyroscopeDeviation _ref_musedatatransformer))) 1e+02) (Variables|Settings|GetRotationSpeed))))))

(event Input|AxisEvents|InputAxisMoveForward
  (params (AxisValue :type Float%20%28single-precision%29))
  ;[1 1 1] MOVEMENT INPUTS
  (Pawn|Input|AddMovementInput (Transformation|GetActorForwardVector) AxisValue false))

(event Input|AxisEvents|InputAxisMoveRight
  (params (AxisValue :type Float%20%28single-precision%29))
  ;[1 1 1] MOVEMENT INPUTS
  (Pawn|Input|AddMovementInput (Transformation|GetActorRightVector) AxisValue false))

(event Input|AxisEvents|InputAxisLookRight
  (params (AxisValue :type Float%20%28single-precision%29))
  ;[1 1 1] MOVEMENT INPUTS
)

(event Input|AxisEvents|InputAxisLookUp
  (params (AxisValue :type Float%20%28single-precision%29))
  ;[1 1 1] MOVEMENT INPUTS
  (Pawn|Input|AddControllerYawInput AxisValue))

(fn ConstructionScript)