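; Helper function library for applying saved audio settings and playing UI sound.
; LoadAudioSettings sets SCM_Master as the base sound mix, then, if the SoundSettings save slot exists, overrides music and SFX class volumes from BP_SaveGame.
; PlayUISound creates and plays the MS_UI 2D sound with persistence across level transitions, so it is not cut off by a map change.
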(fn LoadAudioSettings
  (bind ___worldcontext (LocalVariables|Get__WorldContext))
  (Class|GameplayStatics|SetBaseSoundMix (LocalVariables|Get__WorldContext) "/Game/Audio/Mixes/SCM_Master.SCM_Master")
  (bind _returnvalue (SaveGame|DoesSaveGameExist "SoundSettings"))
  (if _returnvalue
    (bind _returnvalue_2 (SaveGame|LoadGamefromSlot "SoundSettings"))
    (bind _asbp_save_game (Utilities|Casting|CastToBP_SaveGame _returnvalue_2))
    (Audio|SetSoundMixClassOverride ___worldcontext "/Game/Audio/Mixes/SCM_Master.SCM_Master" "/Game/Audio/Classes/SC_Music.SC_Music" (Variables|/Game/Blueprints/BP_SaveGame.BP_SaveGame_C|GetMusicVolume _asbp_save_game) 1.0 1.0 true)
    (Audio|SetSoundMixClassOverride ___worldcontext "/Game/Audio/Mixes/SCM_Master.SCM_Master" "/Game/Audio/Classes/SC_SFX.SC_SFX" (Variables|/Game/Blueprints/BP_SaveGame.BP_SaveGame_C|GetSFXVolume _asbp_save_game) 1.0 1.0 true)))

(fn PlayUISound
  (bind _returnvalue (Audio|CreateSound2D 0 "/Game/Audio/MetaSounds/MS_UI.MS_UI" 1.0 1.0 0.0 0 true))
  (Audio|Components|Audio|Play _returnvalue 0.0))