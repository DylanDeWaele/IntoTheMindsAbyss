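; BP_MuseOSCReceiver receives Muse headband biosensor data over OSC and exposes it to the game.
; On BeginPlay it starts an OSC server on a configurable port, plus a dev HUD in debug mode.
; A switch on message address stores brainwave bands, sensor fit, motion, pulse, battery and mental-state scores.
; Bands, horseshoe, gyroscope, blink and jaw clench also fire events; CalculateFocusLevels is an empty stub.
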(event Custom|On%20OSC%20Message%20Received
  (params (Message :type OSC%20Message%20Structure%20%28by%20ref%29) (IPAddress :type String) (Port :type Integer))
  ;[1 1 1] OSC
  (bind _output_get (Variables|Internal|SetCurrentOSCMessage Message))
  (bind _returnvalue (Class|OSCManager|GetOSCMessageAddress _output_get))
  (bind _returnvalue_2 (Class|OSCManager|GetOSCAddressFullPath _returnvalue))
  (switch string _returnvalue_2
    (:/muse/elements/delta_absolute
      (bind _value (Class|OSCManager|GetFloat (Variables|Internal|GetCurrentOSCMessage)))
      (Variables|Muse|SetDeltaAVG _value)
      (Default|CallOnDeltaOSCReceived))
    (:/muse/elements/theta_absolute
      (bind _value_2 (Class|OSCManager|GetFloat (Variables|Internal|GetCurrentOSCMessage)))
      (Variables|Muse|SetThetaAVG _value_2)
      (Default|CallOnThetaOSCReceived))
    (:/muse/elements/alpha_absolute
      (bind _value_3 (Class|OSCManager|GetFloat (Variables|Internal|GetCurrentOSCMessage)))
      (Variables|Muse|SetAlphaAVG _value_3)
      (Default|CallOnAlphaOSCReceived))
    (:/muse/elements/beta_absolute
      (bind _value_4 (Class|OSCManager|GetFloat (Variables|Internal|GetCurrentOSCMessage)))
      (Variables|Muse|SetBetaAVG _value_4)
      (Default|CallOnBetaOSCReceived))
    (:/muse/elements/gamma_absolute
      (bind _value_5 (Class|OSCManager|GetFloat (Variables|Internal|GetCurrentOSCMessage)))
      (Variables|Muse|SetGammaAVG _value_5)
      (Default|CallOnGammaOSCReceived))
    (:/muse/elements/horseshoe
      (bind _values (Class|OSCManager|GetAllFloats (Variables|Internal|GetCurrentOSCMessage)))
      (for (_array_element _array_index) _values
        (Utilities|Array|SetArrayElem (Variables|Muse|GetHorseshoe) _array_index (Math|Float|Truncate _array_element)))
      (Default|CallOnHorseshoeOSCReceived))
    (:/muse/batt
      (bind _value_6 (Class|OSCManager|GetInt32 (Variables|Internal|GetCurrentOSCMessage)))
      (Variables|Muse|SetBatteryLevel _value_6))
    (:/muse/gyro
      (bind _values_2 (Class|OSCManager|GetAllFloats (Variables|Internal|GetCurrentOSCMessage)))
      (Variables|Muse|SetGyroscope (Math|Vector|MakeVector (Utilities|Array|Get(acopy) _values_2) (Utilities|Array|Get(acopy) _values_2 1) (Utilities|Array|Get(acopy) _values_2 2)))
      (Default|CallOnGyroscopeOSCReceived))
    (:/muse/acc
      (bind _values_3 (Class|OSCManager|GetAllFloats (Variables|Internal|GetCurrentOSCMessage)))
      (Variables|Muse|SetAccelerometer (Math|Vector|MakeVector (Utilities|Array|Get(acopy) _values_3) (Utilities|Array|Get(acopy) _values_3 1) (Utilities|Array|Get(acopy) _values_3 2))))
    (:/muse/elements/blink
      (bind _value_7 (Class|OSCManager|GetInt32 (Variables|Internal|GetCurrentOSCMessage)))
      (if (== _value_7 1)
        (Default|CallOnBlink)))
    (:/muse/elements/jaw_clench
      (bind _value_8 (Class|OSCManager|GetInt32 (Variables|Internal|GetCurrentOSCMessage)))
      (if (== _value_8 1)
        (Default|CallOnJawClench)))
    (:/muse/ppg
      (bind _value_9 (Class|OSCManager|GetFloat (Variables|Internal|GetCurrentOSCMessage) 2))
      (Variables|Muse|SetPulseIR (Math|Float|Truncate (/ _value_9 1e+06))))
    (:/muse/algorithm/mellow
      (bind _value_10 (Class|OSCManager|GetFloat (Variables|Internal|GetCurrentOSCMessage)))
      (Variables|Muse|SetMellow _value_10))
    (:/muse/algorithm/concentration
      (bind _value_11 (Class|OSCManager|GetFloat (Variables|Internal|GetCurrentOSCMessage)))
      (Variables|Muse|SetConcentration _value_11))))

(event EventBeginPlay
  (bind _debug (Variables|Settings|GetDebug))
  (bind _debug_2 (Variables|Settings|GetDebug))
  ;[1 1 1] Begin Play
  (Utilities|FlowControl|Sequence
    (:then_0
      (Development|PrintString "Creating OSC Server" _debug_2 _debug_2)
      (bind _returnvalue (Class|OSCManager|CreateOSCServer "0.0.0.0" (Variables|Settings|Network|GetPort) false true "" 0))
      (bind _output_get (Variables|Internal|SetOSCServer _returnvalue))
      (EventDispatchers|UnbindallEventsfromOnOscMessageReceived _output_get)
      (EventDispatchers|BindEventtoOnOscMessageReceived _output_get (delegate Custom|On%20OSC%20Message%20Received))
      (Development|PrintString "OSC Server created!" _debug _debug))
    (:then_1
      (if (Variables|Settings|GetDebug)
        (bind _returnvalue_2 (UserInterface|CreateWidget "/Game/Widgets/BPW_DevHUD.BPW_DevHUD_C"))
        (UserInterface|Viewport|AddtoViewport _returnvalue_2 1)))))

(fn ConstructionScript)

(fn CalculateFocusLevels)