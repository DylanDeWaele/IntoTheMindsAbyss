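; Turns Muse EEG headset data from BP_MuseOSCReceiver into normalized brainwaves, gyroscope deviation and a scare indicator.
; Baseline calculation requires good horseshoe contact, samples band and gyroscope values over a timed window, and aborts if contact degrades.
; A repeating delay loop then scores each band's range-scaled shift from baseline as a clamped weighted sum.
; The game instance stores the baseline, so later instances restore it and resume scoring on BeginPlay.
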(event Custom|OnGyroscopeOSCReceived
  ;[1 1 1] Array Filling
  (if (Variables|Baselines|GetbIsCalculatingBaseline)
    (Utilities|Array|Add (Variables|Gyroscope|GetGyoscopeArray) (Variables|/Game/Blueprints/Muse/BP_MuseOSCReceiver.BP_MuseOSCReceiver_C|GetGyroscope (Variables|Internal|GetREF_MuseOSCReceiver)))))

(event Custom|OnDeltaReceived
  ;[1 1 1] Array Filling
  (if (or (Variables|Baselines|GetbIsCalculatingBaseline) (Variables|State|GetbIsCalculatingCurrentAverage))
    (Utility|AppendtoArrayifinBounds (Variables|/Game/Blueprints/Muse/BP_MuseOSCReceiver.BP_MuseOSCReceiver_C|GetDeltaAVG (Variables|Internal|GetREF_MuseOSCReceiver)) (Variables|Internal|GetDeltaArray))))

(event Custom|StartScareIndicatorCalculation
  ;[1 1 1] Calculate Scare Indicator
  (Variables|State|SetbIsCalculatingCurrentAverage true)
  (Utilities|FlowControl|Delay (Variables|Settings|GetStateCalculationInterval) :!label _label)
  (ScareIndicator|CalculateScareIndicator)
  (Utility|ClearArrays)
  (if (Variables|State|GetbIsCalculatingCurrentAverage)
    (goto _label)))

(event Custom|OnGammaReceived
  ;[1 1 1] Array Filling
  (if (or (Variables|Baselines|GetbIsCalculatingBaseline) (Variables|State|GetbIsCalculatingCurrentAverage))
    (Utility|AppendtoArrayifinBounds (Variables|/Game/Blueprints/Muse/BP_MuseOSCReceiver.BP_MuseOSCReceiver_C|GetGammaAVG (Variables|Internal|GetREF_MuseOSCReceiver)) (Variables|Internal|GetGammaArray))))

(event Custom|OnThetaReceived
  ;[1 1 1] Array Filling
  (if (or (Variables|Baselines|GetbIsCalculatingBaseline) (Variables|State|GetbIsCalculatingCurrentAverage))
    (Utility|AppendtoArrayifinBounds (Variables|/Game/Blueprints/Muse/BP_MuseOSCReceiver.BP_MuseOSCReceiver_C|GetThetaAVG (Variables|Internal|GetREF_MuseOSCReceiver)) (Variables|Internal|GetThetaArray))))

(event Custom|CalculateBaselinesExternal
  ;[1 0 0] DEBUG - REMOVE
  (CallFunction|StartBaselineCalculation)
  (EventDispatchers|BindEventtoOnBaselineCalculated (delegate Custom|StartScareIndicatorCalculation)))

(event Custom|OnAlphaReceived
  ;[1 1 1] Array Filling
  (if (or (Variables|Baselines|GetbIsCalculatingBaseline) (Variables|State|GetbIsCalculatingCurrentAverage))
    (Utility|AppendtoArrayifinBounds (Variables|/Game/Blueprints/Muse/BP_MuseOSCReceiver.BP_MuseOSCReceiver_C|GetAlphaAVG (Variables|Internal|GetREF_MuseOSCReceiver)) (Variables|Internal|GetAlphaArray))))

(event Custom|StartBaselineCalculation
  (bind _debug (Variables|Settings|GetDebug))
  (bind _debug_2 (Variables|Settings|GetDebug))
  (bind _debug_3 (Variables|Settings|GetDebug))
  ;[1 1 1] Calculating Baseline
  (bind _placedcorrectly (Muse|IsHeadsetPlacedCorrectly))
  (if _placedcorrectly
    (if (not (Variables|Baselines|GetbIsCalculatingBaseline))
      (Development|PrintString "Calculating Baseline..." _debug_3 _debug_3 "(R=0.000000,G=0.982639,B=1.000000,A=1.000000)" (Variables|Settings|GetBaselineCalculationTime))
      (Variables|State|SetbIsCalculatingCurrentAverage false)
      (Utility|ClearArrays)
      (Variables|Baselines|SetbIsCalculatingBaseline true)
      (Utilities|FlowControl|Delay (Variables|Settings|GetBaselineCalculationTime))
      (if (Variables|Baselines|GetbIsCalculatingBaseline)
        (Variables|Baselines|SetbIsCalculatingBaseline false)
        (Baselines|CalculateBaselines)
        (Variables|Baselines|SetbIsBaselineCalculated true)
        (GameInstance|SetDatainGameInstance)
        (Development|PrintString "Baseline Calculated!" _debug _debug "(R=0.000000,G=1.000000,B=0.147884,A=1.000000)")
        (Default|CallOnBaselineCalculated)))
    (else
      (Development|PrintString "Headset not placed correctly!" _debug_2 _debug_2 "(R=1.000000,G=0.000000,B=0.016322,A=1.000000)"))))

(event Custom|OnBetaReceived
  ;[1 1 1] Array Filling
  (if (or (Variables|Baselines|GetbIsCalculatingBaseline) (Variables|State|GetbIsCalculatingCurrentAverage))
    (Utility|AppendtoArrayifinBounds (Variables|/Game/Blueprints/Muse/BP_MuseOSCReceiver.BP_MuseOSCReceiver_C|GetBetaAVG (Variables|Internal|GetREF_MuseOSCReceiver)) (Variables|Internal|GetBetaArray))))

(event Custom|OnHorseshoeReceived
  ;[1 1 1] Array Filling
  (if (Variables|Baselines|GetbIsCalculatingBaseline)
    (bind _placedcorrectly (Muse|IsHeadsetPlacedCorrectly))
    (if (not _placedcorrectly)
      (Baselines|AbortBaselineCalculation)
      (Default|CallOnBaselineCalculationAborted))))

(event EventBeginPlay
  ;[1 1 1] Begin Play
  (GameInstance|GetDatafromGameInstance)
  (bind _returnvalue (Actor|GetActorOfClass "/Game/Blueprints/Muse/BP_MuseOSCReceiver.BP_MuseOSCReceiver_C"))
  (bind _output_get (Variables|Internal|SetREF_MuseOSCReceiver _returnvalue))
  (Utilities|IsValid _output_get
    (:Is%20Valid
      (Init|BindEvents))))

(event EventTick
  (params (DeltaSeconds :type Float%20%28single-precision%29))
  ;[1 1 1] Event Tick
  (Muse|NormalizeBrainwaves)
  (if (Variables|Baselines|GetbIsBaselineCalculated)
    (Gyrosocpe|CalculateGyroscopeDeviation)))

(event Input|KeyboardEvents|C
  (params (Key :type Key%20Structure :default "None"))
  ;[1 0 0] DEBUG - REMOVE
  (:Pressed
    (CallFunction|StartBaselineCalculation)
    (EventDispatchers|BindEventtoOnBaselineCalculated (delegate Custom|StartScareIndicatorCalculation))))

(fn ConstructionScript)

(fn NormalizeBrainwaves
  (bind _ref_museoscreceiver (Variables|Internal|GetREF_MuseOSCReceiver))
  (Variables|Muse|SetDeltaNormalized (Math|Float|NormalizetoRange (Variables|/Game/Blueprints/Muse/BP_MuseOSCReceiver.BP_MuseOSCReceiver_C|GetDeltaAVG _ref_museoscreceiver) -1.0 1.0))
  (Variables|Muse|SetThetaNormalized (Math|Float|NormalizetoRange (Variables|/Game/Blueprints/Muse/BP_MuseOSCReceiver.BP_MuseOSCReceiver_C|GetThetaAVG _ref_museoscreceiver) -1.0 1.0))
  (Variables|Muse|SetAlphaNormalized (Math|Float|NormalizetoRange (Variables|/Game/Blueprints/Muse/BP_MuseOSCReceiver.BP_MuseOSCReceiver_C|GetAlphaAVG _ref_museoscreceiver) -1.0 1.0))
  (Variables|Muse|SetBetaNormalized (Math|Float|NormalizetoRange (Variables|/Game/Blueprints/Muse/BP_MuseOSCReceiver.BP_MuseOSCReceiver_C|GetBetaAVG _ref_museoscreceiver) -1.0 1.0))
  (Variables|Muse|SetGammaNormalized (Math|Float|NormalizetoRange (Variables|/Game/Blueprints/Muse/BP_MuseOSCReceiver.BP_MuseOSCReceiver_C|GetGammaAVG _ref_museoscreceiver) -1.0 1.0)))

(fn CalculateBaselines
  (bind _deltaarray (Variables|Internal|GetDeltaArray))
  (bind _thetaarray (Variables|Internal|GetThetaArray))
  (bind _alphaarray (Variables|Internal|GetAlphaArray))
  (bind _betaarray (Variables|Internal|GetBetaArray))
  (bind _gammaarray (Variables|Internal|GetGammaArray))
  (bind _average (Utility|CalculateAverage _deltaarray))
  (Variables|Baselines|SetDeltaBaseline _average)
  (Variables|Baselines|SetDeltaMin (.MinValue (Math|Float|MinOfFloatArray _deltaarray)))
  (Variables|Baselines|SetDeltaMax (.MaxValue (Math|Float|MaxOfFloatArray _deltaarray)))
  (bind _average_2 (Utility|CalculateAverage _thetaarray))
  (Variables|Baselines|SetThetaBaseline _average_2)
  (Variables|Baselines|SetThetaMin (.MinValue (Math|Float|MinOfFloatArray _thetaarray)))
  (Variables|Baselines|SetThetaMax (.MaxValue (Math|Float|MaxOfFloatArray _thetaarray)))
  (bind _average_3 (Utility|CalculateAverage _alphaarray))
  (Variables|Baselines|SetAlphaBaseline _average_3)
  (Variables|Baselines|SetAlphaMin (.MinValue (Math|Float|MinOfFloatArray _alphaarray)))
  (Variables|Baselines|SetAlphaMax (.MaxValue (Math|Float|MaxOfFloatArray _alphaarray)))
  (bind _average_4 (Utility|CalculateAverage _betaarray))
  (Variables|Baselines|SetBetaBaseline _average_4)
  (Variables|Baselines|SetBetaMin (.MinValue (Math|Float|MinOfFloatArray _betaarray)))
  (Variables|Baselines|SetBetaMax (.MaxValue (Math|Float|MaxOfFloatArray _betaarray)))
  (bind _average_5 (Utility|CalculateAverage _gammaarray))
  (Variables|Baselines|SetGammaBaseline _average_5)
  (Variables|Baselines|SetGammaMin (.MinValue (Math|Float|MinOfFloatArray _gammaarray)))
  (Variables|Baselines|SetGammaMax (.MaxValue (Math|Float|MaxOfFloatArray _gammaarray)))
  (Variables|Gyroscope|SetBaselineGyroscope (Math|Vector|GetVectorArrayAverage (Variables|Gyroscope|GetGyoscopeArray))))

(fn IsHeadsetPlacedCorrectly
  (bind _ref_museoscreceiver (Variables|Internal|GetREF_MuseOSCReceiver))
  (bind _horseshoe (Variables|/Game/Blueprints/Muse/BP_MuseOSCReceiver.BP_MuseOSCReceiver_C|GetHorseshoe _ref_museoscreceiver))
  (bind _output (Utilities|Array|Get(acopy) _horseshoe 3))
  (bind _output_2 (Utilities|Array|Get(acopy) _horseshoe))
  (bind _output_3 (Utilities|Array|Get(acopy) _horseshoe 1))
  (bind _output_4 (Utilities|Array|Get(acopy) _horseshoe 2))
  (return (Math|Boolean|ANDBoolean (and (<= _output_2 2) (> _output_2 0)) (and (<= _output_3 2) (> _output_3 0)) (and (<= _output_4 2) (> _output_4 0)) (and (<= _output 2) (> _output 0)))))

(fn BindEvents
  (bind _ref_museoscreceiver (Variables|Internal|GetREF_MuseOSCReceiver))
  (EventDispatchers|BindEventtoOnDeltaOSCReceived _ref_museoscreceiver (EventDispatchers|CreateEvent :!event Custom|OnDeltaReceived))
  (EventDispatchers|BindEventtoOnThetaOSCReceived _ref_museoscreceiver (EventDispatchers|CreateEvent :!event Custom|OnThetaReceived))
  (EventDispatchers|BindEventtoOnAlphaOSCReceived _ref_museoscreceiver (EventDispatchers|CreateEvent :!event Custom|OnAlphaReceived))
  (EventDispatchers|BindEventtoOnBetaOSCReceived _ref_museoscreceiver (EventDispatchers|CreateEvent :!event Custom|OnBetaReceived))
  (EventDispatchers|BindEventtoOnGammaOSCReceived _ref_museoscreceiver (EventDispatchers|CreateEvent :!event Custom|OnGammaReceived))
  (EventDispatchers|BindEventtoOnHorseshoeOSCReceived _ref_museoscreceiver (EventDispatchers|CreateEvent :!event Custom|OnHorseshoeReceived))
  (EventDispatchers|BindEventtoOnGyroscopeOSCReceived _ref_museoscreceiver (EventDispatchers|CreateEvent :!event Custom|OnGyroscopeOSCReceived)))

(fn IsBetween
  (params (Value :type Float%20%28double-precision%29) (Min :type Float%20%28double-precision%29) (Max :type Float%20%28double-precision%29))
  (return (and (> Value Min) (< Value Max))))

(fn AppendtoArrayifinBounds
  (params (Value :type Float%20%28double-precision%29) (Array :type Array%20of%20Floats%20%28double-precision%29))
  (bind _isbetween (Utility|IsBetween Value -1.0 1.0))
  (if _isbetween
    (Utilities|Array|Add Array Value)
    (return)))

(fn CalculateAverage
  (params (Array :type Array%20of%20Floats%20%28double-precision%29))
  (for _array_element Array
    (LocalVariables|SetSum (+ _array_element (LocalVariables|GetSum))))
  (return (/ (LocalVariables|GetSum) (Math|Conversions|ToFloat(Integer) (Utilities|Array|Length Array)))))

(fn ClearArrays
  (Utilities|Array|Clear (Variables|Internal|GetDeltaArray))
  (Utilities|Array|Clear (Variables|Internal|GetThetaArray))
  (Utilities|Array|Clear (Variables|Internal|GetAlphaArray))
  (Utilities|Array|Clear (Variables|Internal|GetBetaArray))
  (Utilities|Array|Clear (Variables|Internal|GetGammaArray)))

(fn AbortBaselineCalculation
  (Variables|Baselines|SetbIsCalculatingBaseline false)
  (Development|PrintString "Baseline calculation aborted!" true true "(R=1.000000,G=0.007764,B=0.000000,A=1.000000)"))

(fn CalculateScareIndicator
  ;[1 1 1] Calculate Average
  (bind _average (Utility|CalculateAverage (Variables|Internal|GetDeltaArray)))
  (Variables|State|SetCurrentDeltaAVG _average)
  (bind _average_2 (Utility|CalculateAverage (Variables|Internal|GetThetaArray)))
  (Variables|State|SetCurrentThetaAVG _average_2)
  (bind _average_3 (Utility|CalculateAverage (Variables|Internal|GetAlphaArray)))
  (Variables|State|SetCurrentAlphaAVG _average_3)
  (bind _average_4 (Utility|CalculateAverage (Variables|Internal|GetBetaArray)))
  (Variables|State|SetCurrentBetaAVG _average_4)
  (bind _average_5 (Utility|CalculateAverage (Variables|Internal|GetGammaArray)))
  (Variables|State|SetCurrentGammaAVG _average_5)
  ;[1 1 1] Calculate Weighted Average
  (Variables|State|SetScareIndicator (Math|Float|Clamp(Float) (* (+ (* (/ (- (Variables|State|GetCurrentDeltaAVG) (Variables|Baselines|GetDeltaBaseline)) (- (Variables|Baselines|GetDeltaMax) (Variables|Baselines|GetDeltaMin))) (Variables|State|GetDeltaWeight)) (* (/ (- (Variables|State|GetCurrentThetaAVG) (Variables|Baselines|GetThetaBaseline)) (- (Variables|Baselines|GetThetaMax) (Variables|Baselines|GetThetaMin))) (Variables|State|GetThetaWeight)) (* (/ (- (Variables|State|GetCurrentAlphaAVG) (Variables|Baselines|GetAlphaBaseline)) (- (Variables|Baselines|GetAlphaMax) (Variables|Baselines|GetAlphaMin))) (Variables|State|GetAlphaWeight)) (* (/ (- (Variables|State|GetCurrentBetaAVG) (Variables|Baselines|GetBetaBaseline)) (- (Variables|Baselines|GetBetaMax) (Variables|Baselines|GetBetaMin))) (Variables|State|GetBetaWeight)) (* (/ (- (Variables|State|GetCurrentGammaAVG) (Variables|Baselines|GetGammaBaseline)) (- (Variables|Baselines|GetGammaMax) (Variables|Baselines|GetGammaMin))) (Variables|State|GetGammaWeight))) 2.0) 0.0 1e+01)))

(fn CalculateGyroscopeDeviation
  (Variables|Gyroscope|SetGyroscopeDeviation (- (Variables|/Game/Blueprints/Muse/BP_MuseOSCReceiver.BP_MuseOSCReceiver_C|GetGyroscope (Variables|Internal|GetREF_MuseOSCReceiver)) (Variables|Gyroscope|GetBaselineGyroscope))))

(fn GetDatafromGameInstance
  (bind _asbp_game_instance (Utilities|Casting|CastToBP_GameInstance (Game|GetGameInstance)))
  (if (Variables|/Game/Blueprints/Game/BP_GameInstance.BP_GameInstance_C|GetbIsBaselineCalculated _asbp_game_instance)
    (Variables|Baselines|SetbIsBaselineCalculated true)
    (Variables|Gyroscope|SetBaselineGyroscope (Variables|/Game/Blueprints/Game/BP_GameInstance.BP_GameInstance_C|GetBaselineGyroscope _asbp_game_instance))
    (Variables|Baselines|SetDeltaMin (Variables|/Game/Blueprints/Game/BP_GameInstance.BP_GameInstance_C|GetDeltaMin _asbp_game_instance))
    (Variables|Baselines|SetDeltaMax (Variables|/Game/Blueprints/Game/BP_GameInstance.BP_GameInstance_C|GetDeltaMax _asbp_game_instance))
    (Variables|Baselines|SetDeltaBaseline (Variables|/Game/Blueprints/Game/BP_GameInstance.BP_GameInstance_C|GetDeltaBaseline _asbp_game_instance))
    (Variables|Baselines|SetAlphaBaseline (Variables|/Game/Blueprints/Game/BP_GameInstance.BP_GameInstance_C|GetAlphaBaseline _asbp_game_instance))
    (Variables|Baselines|SetAlphaMin (Variables|/Game/Blueprints/Game/BP_GameInstance.BP_GameInstance_C|GetAlphaMin _asbp_game_instance))
    (Variables|Baselines|SetAlphaMax (Variables|/Game/Blueprints/Game/BP_GameInstance.BP_GameInstance_C|GetAlphaMax _asbp_game_instance))
    (Variables|Baselines|SetThetaBaseline (Variables|/Game/Blueprints/Game/BP_GameInstance.BP_GameInstance_C|GetThetaBaseline _asbp_game_instance))
    (Variables|Baselines|SetThetaMax (Variables|/Game/Blueprints/Game/BP_GameInstance.BP_GameInstance_C|GetThetaMax _asbp_game_instance))
    (Variables|Baselines|SetThetaMin (Variables|/Game/Blueprints/Game/BP_GameInstance.BP_GameInstance_C|GetThetaMin _asbp_game_instance))
    (Variables|Baselines|SetBetaBaseline (Variables|/Game/Blueprints/Game/BP_GameInstance.BP_GameInstance_C|GetBetaBaseline _asbp_game_instance))
    (Variables|Baselines|SetBetaMin (Variables|/Game/Blueprints/Game/BP_GameInstance.BP_GameInstance_C|GetBetaMin _asbp_game_instance))
    (Variables|Baselines|SetBetaMax (Variables|/Game/Blueprints/Game/BP_GameInstance.BP_GameInstance_C|GetBetaMax _asbp_game_instance))
    (Variables|Baselines|SetGammaBaseline (Variables|/Game/Blueprints/Game/BP_GameInstance.BP_GameInstance_C|GetGammaBaseline _asbp_game_instance))
    (Variables|Baselines|SetGammaMin (Variables|/Game/Blueprints/Game/BP_GameInstance.BP_GameInstance_C|GetGammaMin _asbp_game_instance))
    (Variables|Baselines|SetGammaMax (Variables|/Game/Blueprints/Game/BP_GameInstance.BP_GameInstance_C|GetGammaMax _asbp_game_instance))
    (Default|CallOnBaselineCalculated)
    (CallFunction|StartScareIndicatorCalculation)
    (else
      (return))))

(fn SetDatainGameInstance
  (bind _asbp_game_instance (Utilities|Casting|CastToBP_GameInstance (Game|GetGameInstance)))
  (Variables|/Game/Blueprints/Game/BP_GameInstance.BP_GameInstance_C|SetbIsBaselineCalculated _asbp_game_instance (Variables|Baselines|GetbIsBaselineCalculated))
  (Variables|/Game/Blueprints/Game/BP_GameInstance.BP_GameInstance_C|SetBaselineGyroscope _asbp_game_instance (Variables|Gyroscope|GetBaselineGyroscope))
  (Variables|/Game/Blueprints/Game/BP_GameInstance.BP_GameInstance_C|SetAlphaBaseline _asbp_game_instance (Variables|Baselines|GetAlphaBaseline))
  (Variables|/Game/Blueprints/Game/BP_GameInstance.BP_GameInstance_C|SetAlphaMax _asbp_game_instance (Variables|Baselines|GetAlphaMax))
  (Variables|/Game/Blueprints/Game/BP_GameInstance.BP_GameInstance_C|SetAlphaMin _asbp_game_instance (Variables|Baselines|GetAlphaMin))
  (Variables|/Game/Blueprints/Game/BP_GameInstance.BP_GameInstance_C|SetDeltaBaseline _asbp_game_instance (Variables|Baselines|GetDeltaBaseline))
  (Variables|/Game/Blueprints/Game/BP_GameInstance.BP_GameInstance_C|SetDeltaMin _asbp_game_instance (Variables|Baselines|GetDeltaMin))
  (Variables|/Game/Blueprints/Game/BP_GameInstance.BP_GameInstance_C|SetDeltaMax _asbp_game_instance (Variables|Baselines|GetDeltaMax))
  (Variables|/Game/Blueprints/Game/BP_GameInstance.BP_GameInstance_C|SetThetaBaseline _asbp_game_instance (Variables|Baselines|GetThetaBaseline))
  (Variables|/Game/Blueprints/Game/BP_GameInstance.BP_GameInstance_C|SetThetaMin _asbp_game_instance (Variables|Baselines|GetThetaMin))
  (Variables|/Game/Blueprints/Game/BP_GameInstance.BP_GameInstance_C|SetThetaMax _asbp_game_instance (Variables|Baselines|GetThetaMax))
  (Variables|/Game/Blueprints/Game/BP_GameInstance.BP_GameInstance_C|SetBetaMin _asbp_game_instance (Variables|Baselines|GetBetaMin))
  (Variables|/Game/Blueprints/Game/BP_GameInstance.BP_GameInstance_C|SetBetaMax _asbp_game_instance (Variables|Baselines|GetBetaMax))
  (Variables|/Game/Blueprints/Game/BP_GameInstance.BP_GameInstance_C|SetBetaBaseline _asbp_game_instance (Variables|Baselines|GetBetaBaseline))
  (Variables|/Game/Blueprints/Game/BP_GameInstance.BP_GameInstance_C|SetGammaMax _asbp_game_instance (Variables|Baselines|GetGammaMax))
  (Variables|/Game/Blueprints/Game/BP_GameInstance.BP_GameInstance_C|SetGammaBaseline _asbp_game_instance (Variables|Baselines|GetGammaBaseline))
  (Variables|/Game/Blueprints/Game/BP_GameInstance.BP_GameInstance_C|SetGammaMin _asbp_game_instance (Variables|Baselines|GetGammaMin)))