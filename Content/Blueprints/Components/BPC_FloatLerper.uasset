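; BPC_FloatLerper is a component that eases a float Value toward a Target over time.
; SetTarget stores the old target, so Tick detects a change and restarts Alpha from the current Value.
; Later ticks advance Alpha by delta time times LerpSpeed and lerp linearly, so transition time is independent of distance.
; IsLerping stays true while Value differs from Target.
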(event EventTick
  (params (DeltaSeconds :type Float%20%28single-precision%29))
  (bind _output_get (Variables|Values|SetbIsLerping (not (== (Variables|Values|GetValue) (Variables|Internal|GetTarget)))))
  (if _output_get
    (if (== (Variables|Internal|GetTarget) (Variables|Internal|GetPreviousTarget))
      (bind _output_get_2 (Variables|Internal|SetAlpha (Math|Float|Clamp(Float) (+ (* (Utilities|Time|GetWorldDeltaSeconds) (Variables|Settings|GetLerpSpeed)) (Variables|Internal|GetAlpha)))))
      (Variables|Values|SetValue (Math|Float|Lerp (Variables|Internal|GetPreviousValue) (Variables|Internal|GetTarget) _output_get_2))
      (else
        (Variables|Internal|SetAlpha 0.0)
        (Variables|Internal|SetPreviousValue (Variables|Values|GetValue))
        (Variables|Internal|SetPreviousTarget (Variables|Internal|GetTarget))))))

(fn SetTarget
  (params (NewTarget :type Float%20%28double-precision%29))
  (Variables|Internal|SetPreviousTarget (Variables|Internal|GetTarget))
  (Variables|Internal|SetTarget NewTarget))