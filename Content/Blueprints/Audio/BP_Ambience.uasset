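; Ambience actor that drives adaptive audio from Muse EEG brainwave data, starting playback on BeginPlay unless muted.
; Each tick it reads BP_MuseDataTransformer to target lerpers for binaural frequency (chosen by the dominant normalized band), scare indicator and five band averages.
; Values of lerpers still interpolating are written to the Ambience sound's float parameters.
; A debug key sets a random binaural target.
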(event EventBeginPlay
  ;[1 1 1] Begin Play
  (bind _returnvalue (Actor|GetActorOfClass "/Game/Blueprints/Muse/BP_MuseDataTransformer.BP_MuseDataTransformer_C"))
  (Variables|Internal|SetREF_MuseDataTransformer _returnvalue)
  (if (not (Variables|Settings|GetbMute))
    (Audio|Components|Audio|Play (Variables|Default|GetAmbience) 0.0)))

(event EventTick
  (params (DeltaSeconds :type Float%20%28single-precision%29))
  ;[1 1 1] Tick
  (Utilities|FlowControl|Sequence
    (:then_0
      (Targets|SetTargetBinauralFrequency)
      (Metasounds|SetAmbienceParameter (Variables|Default|GetBinauralFrequencyLerper) "BinauralFrequency"))
    (:then_1
      (Targets|SetTargetScareIndicator)
      (Metasounds|SetAmbienceParameter (Variables|Default|GetScareIndicatorLerper) "ScareIndicator"))
    (:then_2
      (Targets|SetTargetBrainwaves)
      (Metasounds|SetBrainwaveParameters))))

(event Input|KeyboardEvents|0
  (params (Key :type Key%20Structure))
  (bind _returnvalue (Math|Random|RandomFloatinRange 0.0 4e+01))
  ;[1 1 1] DEBUGGING
  (:Pressed
    (Development|PrintString (Utilities|String|Append (Utilities|String|MakeLiteralString "DEBUG - SET TARGET: ") (Utilities|String|ToString(Float) _returnvalue)))
    (Default|SetTarget (Variables|Default|GetBinauralFrequencyLerper) _returnvalue)))

(fn ConstructionScript)

(fn SetTargetBinauralFrequency
  (bind _binauralfrequencylerper (Variables|Default|GetBinauralFrequencyLerper))
  (bind _ref_musedatatransformer (Variables|Internal|GetREF_MuseDataTransformer))
  (switch int (.IndexOfMaxValue (Math|Float|MaxOfFloatArray (Utilities|Array|MakeArray (Variables|/Game/Blueprints/Muse/BP_MuseDataTransformer.BP_MuseDataTransformer_C|GetDeltaNormalized _ref_musedatatransformer) (Variables|/Game/Blueprints/Muse/BP_MuseDataTransformer.BP_MuseDataTransformer_C|GetThetaNormalized _ref_musedatatransformer) (Variables|/Game/Blueprints/Muse/BP_MuseDataTransformer.BP_MuseDataTransformer_C|GetAlphaNormalized _ref_musedatatransformer) (Variables|/Game/Blueprints/Muse/BP_MuseDataTransformer.BP_MuseDataTransformer_C|GetBetaNormalized _ref_musedatatransformer) (Variables|/Game/Blueprints/Muse/BP_MuseDataTransformer.BP_MuseDataTransformer_C|GetGammaNormalized _ref_musedatatransformer))))
    (:0
      (Default|SetTarget _binauralfrequencylerper 3.0))
    (:1
      (Default|SetTarget _binauralfrequencylerper 7.0))
    (:2
      (Default|SetTarget _binauralfrequencylerper 11.0))
    (:3
      (Default|SetTarget _binauralfrequencylerper 21.0))
    (:4
      (Default|SetTarget _binauralfrequencylerper 37.0))))

(fn SetTargetScareIndicator
  (Default|SetTarget (Variables|Default|GetScareIndicatorLerper) (Variables|/Game/Blueprints/Muse/BP_MuseDataTransformer.BP_MuseDataTransformer_C|GetScareIndicator (Variables|Internal|GetREF_MuseDataTransformer))))

(fn SetAmbienceParameter
  (params (Lerper :type BPC%20Float%20Lerper%20Object%20Reference) (Parameter%20Name :type Name))
  (if (Variables|/Game/Blueprints/Components/BPC_FloatLerper.BPC_FloatLerper_C|GetbIsLerping Lerper)
    (Audio|Parameter|SetFloatParameter (Variables|Default|GetAmbience) Parameter%20Name (Variables|/Game/Blueprints/Components/BPC_FloatLerper.BPC_FloatLerper_C|GetValue Lerper) :!class /Script/AudioExtensions.AudioParameterControllerInterface)))

(fn SetTargetBrainwaves
  (bind _ref_musedatatransformer (Variables|Internal|GetREF_MuseDataTransformer))
  (Default|SetTarget (Variables|Default|GetDeltaLerper) (Variables|/Game/Blueprints/Muse/BP_MuseDataTransformer.BP_MuseDataTransformer_C|GetCurrentDeltaAVG _ref_musedatatransformer))
  (Default|SetTarget (Variables|Default|GetThetaLerper) (Variables|/Game/Blueprints/Muse/BP_MuseDataTransformer.BP_MuseDataTransformer_C|GetCurrentThetaAVG _ref_musedatatransformer))
  (Default|SetTarget (Variables|Default|GetAlphaLerper) (Variables|/Game/Blueprints/Muse/BP_MuseDataTransformer.BP_MuseDataTransformer_C|GetCurrentAlphaAVG _ref_musedatatransformer))
  (Default|SetTarget (Variables|Default|GetBetaLerper) (Variables|/Game/Blueprints/Muse/BP_MuseDataTransformer.BP_MuseDataTransformer_C|GetCurrentBetaAVG _ref_musedatatransformer))
  (Default|SetTarget (Variables|Default|GetGammaLerper) (Variables|/Game/Blueprints/Muse/BP_MuseDataTransformer.BP_MuseDataTransformer_C|GetCurrentGammaAVG _ref_musedatatransformer)))

(fn SetBrainwaveParameters
  (Metasounds|SetAmbienceParameter (Variables|Default|GetDeltaLerper) "DeltaWaves")
  (Metasounds|SetAmbienceParameter (Variables|Default|GetThetaLerper) "ThetaWaves")
  (Metasounds|SetAmbienceParameter (Variables|Default|GetAlphaLerper) "AlphaWaves")
  (Metasounds|SetAmbienceParameter (Variables|Default|GetBetaLerper) "BetaWaves")
  (Metasounds|SetAmbienceParameter (Variables|Default|GetGammaLerper) "GammaWaves"))